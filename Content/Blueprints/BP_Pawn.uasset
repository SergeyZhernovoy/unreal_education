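; BP_Pawn is a player-controlled pawn that slides along the X axis and spawns a ball, like a paddle.
; On BeginPlay it spawns a BP_Ball at its capsule's transform and stores it in PlayingBall.
; Two MoveRight axis events, one per direction, apply a swept fixed-step world offset based only on the input's sign, without delta-time scaling.
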(event EventBeginPlay
  (bind _returnvalue (Game|SpawnActorfromClass "/Game/Blueprints/BP_Ball.BP_Ball_C" (Transformation|GetWorldTransform (Variables|Default|GetCapsule)) "AlwaysSpawn" 0 0))
  (Variables|Default|SetPlayingBall _returnvalue))

(event Collision|EventActorBeginOverlap
  (params (OtherActor :type Actor%20Object%20Reference)))

(event EventTick
  (params (DeltaSeconds :type Float%20%28single-precision%29)))

(event Input|AxisEvents|InputAxisMoveRight
  (params (AxisValue :type Float%20%28single-precision%29))
  (if (> AxisValue 0.0)
    (bind _sweephitresult (Transformation|AddActorWorldOffset "50.000000,0.000000, 0" true))
    (if true
      _)))

(event Input|AxisEvents|InputAxisMoveRight
  (params (AxisValue :type Float%20%28single-precision%29))
  (if (< AxisValue 0.0)
    (bind _sweephitresult (Transformation|AddActorWorldOffset "-50.000000,0.000000, 0" true))
    (if true
      _)))

(fn ConstructionScript)