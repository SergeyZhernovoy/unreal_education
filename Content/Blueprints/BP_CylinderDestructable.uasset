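; BP_CylinderDestructable is an actor with a cylinder component that changes appearance the first time another actor overlaps it.
; On overlap it calls the parent handler, then a FirstCollision flag gates a one-time swap of the cylinder's material to M_Brick_Clay_New.
; Despite the name, its graphs hold no destruction logic, and BeginPlay and Tick are disabled stubs.
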(event EventBeginPlay
  (|CallParentFunction) ; This node is disabled and will not be called.\nDrag off pins to build functionality.
)

(event Collision|EventActorBeginOverlap
  (params (OtherActor :type Actor%20Object%20Reference))
  (|CallParentFunction OtherActor)
  (if (Variables|Default|GetFirstCollision)
    (Rendering|Material|SetMaterial (Variables|Default|GetCylinder) 0 "/Game/StarterContent/Materials/M_Brick_Clay_New.M_Brick_Clay_New")
    (Variables|Default|SetFirstCollision false)))

(event EventTick
  (params (DeltaSeconds :type Float%20%28single-precision%29))
  (|CallParentFunction DeltaSeconds) ; This node is disabled and will not be called.\nDrag off pins to build functionality.
)

(fn ConstructionScript
  (|CallParentFunction))