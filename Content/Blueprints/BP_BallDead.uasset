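; BP_BallDead is a functional test that checks the playing ball dies only at a lower X than the player pawn's cube.
; PrepareTest caches the cube's world location and the pawn's PlayingBall, then binds to that ball's OnDead dispatcher.
; When OnDead fires, the test succeeds if the ball sphere's X is below the cached cube X, and otherwise finishes with an error.
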(event Custom|OnDeadReaction
  (if (< (.x (Transformation|GetWorldLocation (Variables|/Game/Blueprints/BP_Ball.BP_Ball_C|GetSphere (Variables|Default|GetBall)))) (.x (Variables|Default|GetPawnLocation)))
    (Class|FunctionalTest|FinishTest "Succeeded")
    (else
      (Class|FunctionalTest|FinishTest "Error"))))

(event EventPrepareTest
  (bind _asbp_pawn (Utilities|Casting|CastToBP_Pawn (Game|Player|GetPlayerPawn 0)))
  (Variables|Default|SetPawnLocation (Transformation|GetWorldLocation (Variables|/Game/Blueprints/BP_Pawn.BP_Pawn_C|GetCube _asbp_pawn)))
  (bind _output_get (Variables|Default|SetBall (Variables|/Game/Blueprints/BP_Pawn.BP_Pawn_C|GetPlayingBall _asbp_pawn)))
  (EventDispatchers|AssignOnDead _output_get (delegate Custom|OnDeadReaction)))

(event EventStartTest)

(event EventTick
  (params (DeltaSeconds :type Float%20%28single-precision%29)))

(fn ConstructionScript)